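; BP_EnemyCharacter is the enemy character in a Pac-Man style game, resolving who dies when it touches the player.
; On KillingCollision overlap, it skips dead enemies using the PacmanEnemyController state and checks the ThirdPersonCharacter's PacmanState.
; A chasing player kills the enemy through its controller, an already dead player is ignored, and otherwise the player dies.
; Each kill plays its own 2D death sound.
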(event OnComponentBeginOverlap(KillingCollision)
  (params (OverlappedComponent :type Primitive%20Component%20Object%20Reference) (OtherActor :type Actor%20Object%20Reference) (OtherComp :type Primitive%20Component%20Object%20Reference) (OtherBodyIndex :type Integer) (bFromSweep :type Boolean) (SweepResult :type Hit%20Result%20Structure%20%28by%20ref%29))
  (bind _aspacman_enemy_controller (Utilities|Casting|CastToPacmanEnemyController (Pawn|GetController)))
  (if (Utilities|Enum|NotEqual(Enum) (Variables|/Script/Pacman.PacmanEnemyController|GetEnemyState _aspacman_enemy_controller) "Death")
    (bind _asthird_person_character (Utilities|Casting|CastToThirdPersonCharacter OtherActor))
    (if (or (Utilities|Enum|Equal(Enum) (Variables|/Script/Pacman.PacmanCharacter|GetPacmanState _asthird_person_character) "Chasing") (Utilities|Enum|Equal(Enum) (Variables|/Script/Pacman.PacmanCharacter|GetPacmanState _asthird_person_character) "Death"))
      (if (Utilities|Enum|Equal(Enum) (Variables|/Script/Pacman.PacmanCharacter|GetPacmanState _asthird_person_character) "Chasing")
        ;[1 1 1] Enemy death
        (bind _aspacman_enemy_controller_2 (Utilities|Casting|CastToPacmanEnemyController (Pawn|GetController)))
        (Class|PacmanEnemyController|Die _aspacman_enemy_controller_2)
        (bind _returnvalue (Audio|CreateSound2D "/Game/SFX/DeadZombie.DeadZombie" 1.0 1.0 0.0 0))
        (Audio|Components|Audio|Play _returnvalue 0.0))
      (else
        ;[1 1 1] Player death
        (Class|PacmanCharacter|Die _asthird_person_character)
        (bind _returnvalue_2 (Audio|CreateSound2D "/Game/SFX/DeadPlayer.DeadPlayer" 1.0 1.0 0.0 0))
        (Audio|Components|Audio|Play _returnvalue_2 0.0)))))

(event EventBeginPlay)

(event Collision|EventActorBeginOverlap
  (params (OtherActor :type Actor%20Object%20Reference)))

(event EventTick
  (params (DeltaSeconds :type Float%20%28single-precision%29)))

(fn ConstructionScript)