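; BP_Item is an item actor that swings its mesh back and forth and plays an eating sound when destroyed.
; Tick rotates ItemMesh by a fixed per-frame step, not scaled by delta time, while a Delay and FlipFlop reverse the direction about every second.
; BeginPlay binds PlaySound to OnDestroyed, which creates a 2D EatPizza sound, starts it and schedules a stop shortly after.
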(event Custom|PlaySound
  (params (DestroyedActor :type Actor%20Object%20Reference))
  (bind _returnvalue (Audio|CreateSound2D "/Game/SFX/eatPizza.eatPizza" 1.0 1.0 0.0 0))
  (Audio|Components|Audio|Play _returnvalue 0.2)
  (Audio|Components|Audio|StopDelayed _returnvalue 0.5))

(event EventBeginPlay
  (Game|BindEventtoOnDestroyed (delegate Custom|PlaySound)))

(event Collision|EventActorBeginOverlap
  (params (OtherActor :type Actor%20Object%20Reference)))

(event EventTick
  (params (DeltaSeconds :type Float%20%28single-precision%29))
  (Utilities|FlowControl|Sequence
    (:then_0
      (switch int (Variables|Default|GetMultigateIndex)
        (:0
          (Transformation|AddLocalRotation (Variables|Default|GetItemMesh) "0.500000,0.000000,0.000000" false false))
        (:1
          (Transformation|AddLocalRotation (Variables|Default|GetItemMesh) "-0.500000,0.000000, 0" false false))))
    (:then_2
      (Utilities|FlowControl|Delay 1.0)
      (Utilities|FlowControl|FlipFlop
        (:A
          (Variables|Default|SetMultigateIndex 1))
        (:B
          (Variables|Default|SetMultigateIndex 0))))))

(fn ConstructionScript)