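; Pac-Man style power-up actor that turns the chase around when it is destroyed.
; Its OnDestroyed handler, bound at BeginPlay, plays a short 2D sound, sets every PacmanEnemyController to Afraid and switches the player's ThirdPersonCharacter to Chasing.
; Tick spins the item mesh by a fixed step per frame, independent of delta time.
; The actor holds no overlap or destroy logic of its own.
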(event Custom|PlaySound
  (params (DestroyedActor :type Actor%20Object%20Reference))
  (bind _returnvalue (Audio|CreateSound2D 0 1.0 1.0 0.0 0))
  (Audio|Components|Audio|Play _returnvalue 0.2)
  (Audio|Components|Audio|StopDelayed _returnvalue 0.5)
  (Utilities|FlowControl|Sequence
    (:then_0
      (bind _outactors (Actor|GetAllActorsOfClass "/Script/Pacman.PacmanEnemyController"))
      (for _array_element _outactors
        (Class|PacmanEnemyController|ChangeEnemyState _array_element "Afraid")))
    (:then_1
      (bind _asthird_person_character (Utilities|Casting|CastToThirdPersonCharacter (Game|GetPlayerCharacter 0)))
      (Class|PacmanCharacter|ChangePacmanState _asthird_person_character "Chasing"))))

(event EventBeginPlay
  (Game|BindEventtoOnDestroyed (delegate Custom|PlaySound)))

(event EventTick
  (params (DeltaSeconds :type Float%20%28single-precision%29))
  (Transformation|AddLocalRotation (Variables|Default|GetItemMesh) "0.000000,0.200000,0.000000" false false))

(fn ConstructionScript)